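; BP_Exit is an exit marker that removes AI-controlled pawns from the simulation when they reach it.
; On BeginPlay it copies the actor count from the GI_ActorNumbers game instance into its own variable.
; Box overlap destroys the overlapping actor's AI-controlled pawn, decrements that local count and writes it to the Stats text in the BP_SimulationGameMode GUI.
; The game instance's count is never updated.
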(event OnComponentBeginOverlap(Box)
  (params (OverlappedComponent :type Primitive%20Component%20Object%20Reference) (OtherActor :type Actor%20Object%20Reference) (OtherComp :type Primitive%20Component%20Object%20Reference) (OtherBodyIndex :type Integer) (bFromSweep :type Boolean) (SweepResult :type Hit%20Result%20Structure%20%28by%20ref%29))
  (Actor|DestroyActor (Pawn|GetControlledPawn (AI|GetAIController OtherActor)))
  (bind _asbp_simulation_game_mode (Utilities|Casting|CastToBP_SimulationGameMode (Game|GetGameMode)))
  (bind _result (Math|Integer|DecrementInt (Variables|Default|GetActors))
    (:%20%20
      (Variables|/Script/UMG.TextBlock|SetText (Variables|/Game/Main/Blueprints/UI/Widgets/UI/WBP_UserInteface.WBP_UserInteface_C|GetStats (Variables|/Game/Main/Blueprints/GameMode/BP_SimulationGameMode.BP_SimulationGameMode_C|GetGUI _asbp_simulation_game_mode)) (Utilities|Text|ToText(Integer) _result)))))

(event EventBeginPlay
  (bind _asgi_actor_numbers (Utilities|Casting|CastToGI_ActorNumbers (Game|GetGameInstance)))
  (Variables|Default|SetActors (Variables|/Game/Main/Blueprints/GameMode/GameInstance/GI_ActorNumbers.GI_ActorNumbers_C|GetActorNumber _asgi_actor_numbers)))

(event Collision|EventActorBeginOverlap
  (params (OtherActor :type Actor%20Object%20Reference)))

(event EventTick
  (params (DeltaSeconds :type Float%20%28single-precision%29)))

(fn ConstructionScript)