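; BP_MarkArrow is an arrow mark actor that works out the world location it points at.
; On BeginPlay, MarkPointer runs a visibility line trace along the StaticMesh forward vector, with debug drawing left on.
; It stores the impact point in PointingLocation, or the far end of the trace when nothing is hit.
; Its construction script only calls the parent's.
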(event EventBeginPlay
  (CallFunction|MarkPointer))

(fn ConstructionScript
  (|CallParentFunction))

(fn MarkPointer
  (bind _returnvalue (Transformation|GetActorLocation))
  (bind _staticmesh (Variables|Default|GetStaticMesh))
  (bind _returnvalue_2 (Math|Vector|GetForwardVector _staticmesh))
  (bind _returnvalue_3 (* _returnvalue_2 5e+03))
  (bind _returnvalue_4 (+ _returnvalue _returnvalue_3))
  (bind _outhit (Collision|LineTraceByChannel _returnvalue _returnvalue_4 "TraceTypeQuery1" false 0 "ForDuration" true "(R=1.000000,G=0.000000,B=0.000000,A=1.000000)" "(R=0.000000,G=1.000000,B=0.000000,A=1.000000)" 1e+01))
  (if (.bBlockingHit (Collision|BreakHitResult _outhit))
    (Variables|Default|SetPointing%20Location (.ImpactPoint (Collision|BreakHitResult _outhit)))
    (else
      (Variables|Default|SetPointing%20Location _returnvalue_4))))